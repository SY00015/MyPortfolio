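; BP_RandomPointBox is a spawner actor that periodically drops a TrickyPickup at a random point inside its Box volume.
; Tick lowers a countdown by a fixed step, so the spawn interval depends on frame rate rather than elapsed time.
; When the countdown expires, it picks a point within the Box extent around the root component's location, spawns the pickup and resets the countdown.
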(event EventBeginPlay)

(event Collision|EventActorBeginOverlap
  (params (OtherActor :type Actor%20Object%20Reference)))

(event EventTick
  (params (DeltaSeconds :type Float%20%28single-precision%29))
  (Variables|Default|SetcountDown (- (Variables|Default|GetcountDown) 0.1))
  (if (<= (Variables|Default|GetcountDown) 0.0)
    (Game|SpawnActorfromClass "/Script/A1.TrickyPickup" (Math|Conversions|ToTransform(Vector) (Math|Random|RandomPointinBoundingBox (Transformation|GetWorldLocation (Variables|Default|GetDefaultSceneRoot)) (Variables|/Script/Engine.BoxComponent|GetBoxExtent (Variables|Default|GetBox)))) "Undefined" 0 0)
    (Variables|Default|SetcountDown 8.0)))

(fn ConstructionScript)