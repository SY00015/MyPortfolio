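; BP_FindPathPoint is a behavior tree task that looks up the current patrol point for a BP_EnemyPatroler.
; It reads the path index from the Blackboard, takes that entry from the pawn's PatrolPath points and transforms it from local to world space.
; The result is written to the path vector key and the task finishes successfully.
; A failed cast or invalid path never calls FinishExecute.
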(event EventReceiveExecuteAI
  (params (OwnerController :type AI%20Controller%20Object%20Reference) (ControlledPawn :type Pawn%20Object%20Reference))
  (bind _asbp_enemy_patroler (Utilities|Casting|CastToBP_EnemyPatroler ControlledPawn))
  (bind _patrolpath (Variables|/Game/BP_EnemyPatroler.BP_EnemyPatroler_C|GetPatrolPath _asbp_enemy_patroler)
    (:then
      (AI|BehaviorTree|SetBlackboardValueasVector (Variables|Default|GetBB_PathVector) (Math|Transform|TransformLocation (Transformation|GetActorTransform _patrolpath) (Utilities|Array|Get(acopy) (Variables|/Game/BP_PatrolPath.BP_PatrolPath_C|GetPathPoints _patrolpath) (Class|BTFunctionLibrary|GetBlackboardValueasInt (Variables|Default|GetBB_PathIndex)))))
      (AI|BehaviorTree|FinishExecute true))
    (:else)))